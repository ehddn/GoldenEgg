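; BP_MeleeSword is an enemy melee sword that damages the player's avatar on contact.
; When ProxBox begins overlapping an actor of exactly the BP_Avatar class, it calls ToDamage.
; ToDamage casts player character 0 to BP_Avatar and subtracts Damage directly from its Hp, rather than using the overlapped actor.
; An Hp zero check and an unhide node sit unconnected and never run.
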(event `self.ProxBox.OnComponentBeginOverlap`
  (params (OverlappedComponent :type "PrimitiveComponent Object Reference") (OtherActor :type "Actor Object Reference") (OtherComp :type "PrimitiveComponent Object Reference") (OtherBodyIndex :type Integer) (bFromSweep :type Boolean) (SweepResult :type "HitResult Structure (by ref)"))
  (if (== (`GameplayStatics.GetObjectClass` OtherActor) "/Game/Blueprints/BP_Avatar.BP_Avatar_C")
    (`self.ToDamage`)))

(fn `ToDamage`
  (bind _asbp_avatar (cast `/Game/Blueprints/BP_Avatar` (`GameplayStatics.GetPlayerCharacter` 0)))
  (set `Avatar.Hp` (- (`Avatar.Hp` _asbp_avatar) (`self.Damage`)) _asbp_avatar))

(fn `UserConstructionScript`)